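; Dual-mode first-person gun that fires carrot projectiles and applies a vacuum-like absorb force to retrievable objects.
; Shoot checks and spends ammo, spawning BP_CarrotBullet along the camera's aim with montage and sound.
; StartAbsorbing and StopAbsorbing toggle Tick, which sphere-traces the "Retrievable" profile and pushes hits owning BP_RetrieveComponent along their hit normal.
; Absorb still has debug drawing and printing, and its curve-based vector math is unconnected.
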(event `self.ReceiveTick`
  (params (DeltaSeconds :type "Float (single-precision)"))
  (`self.Absorb` DeltaSeconds))

(fn `Absorb`
  (params (DeltaTime :type "Float (double-precision)"))
  (bind _returnvalue (`SceneComponent.K2_GetComponentLocation` (`self.ProjectileSpawnPos`)))
  (set `self.ElapsedTime` (+ DeltaTime (`self.ElapsedTime`)))
  (`AnimInstance.Montage_Play` (`SkeletalMeshComponent.GetAnimInstance` (`self.PlayerArms`)) "/Game/FirstPerson/Animations/FirstPersonFire_Montage.FirstPersonFire_Montage" 1.0 "MontageLength" 0.0 true)
  (bind _outhits (`KismetSystemLibrary.SphereTraceMultiByProfile` _returnvalue (+ _returnvalue (* (`KismetMathLibrary.GreaterGreater_VectorRotator` (`self.GunOffset`) (`SceneComponent.K2_GetComponentRotation` (`self.PlayerCamera`))) (`self.AbsorbRange`))) (`self.AbsorbRadius`) "Retrievable" false (`|MakeArray` (`self.GetParentActor`)) "ForOneFrame"))
  (for (_array_element _array_index) _outhits
    (bind (_bblockinghit _binitialoverlap _time _distance _location _impactpoint _normal _impactnormal _physmat _hitactor _hitcomponent _hitbonename _hititem _faceindex _tracestart _traceend) (`GameplayStatics.BreakHitResult` _array_element))
    (`/Engine/EditorBlueprintResources/StandardMacros.IsValid` (`self.GetComponentByClass` _hitactor "/Game/FarmFight/BP/BP_RetrieveComponent.BP_RetrieveComponent_C")
      (:`Is Valid`
        (`PrimitiveComponent.AddImpulse` _hitcomponent (* _normal (`self.AbsorbStrenght`)) "None" false))))
  (`KismetSystemLibrary.PrintString` (`KismetStringLibrary.Conv_IntToString` _array_index)))

(fn `CanShoot`
  (returns (ReturnValue :type Boolean))
  (return (> (`self.CurrentAmmo`) 0)))

(fn `Shoot`
  (params (Arms :type "SkeletalMeshComponent Object Reference") (Camera :type "CameraComponent Object Reference"))
  (bind _returnvalue (`SceneComponent.K2_GetComponentRotation` Camera))
  (bind _returnvalue_2 (`self.CanShoot`))
  (if _returnvalue_2
    (`AnimInstance.Montage_Play` (`SkeletalMeshComponent.GetAnimInstance` Arms) "/Game/FirstPerson/Animations/FirstPersonFire_Montage.FirstPersonFire_Montage" 1.0 "MontageLength" 0.0 true)
    (`|SpawnActorFromClass` "/Game/FarmFight/BP/BP_CarrotBullet.BP_CarrotBullet_C" (`KismetMathLibrary.MakeTransform` (+ (`SceneComponent.K2_GetComponentLocation` (`self.ProjectileSpawnPos`)) (`KismetMathLibrary.GreaterGreater_VectorRotator` (`self.GunOffset`) _returnvalue)) _returnvalue) "AdjustIfPossibleButDontSpawnIfColliding" "OverrideRootScale" null null) ; Spawn projectile
    (`GameplayStatics.PlaySoundAtLocation` "/Game/FirstPerson/Audio/FirstPersonTemplateWeaponFire02.FirstPersonTemplateWeaponFire02" (`self.K2_GetActorLocation`) (struct) 1.0 1.0 0.0 null null null) ; Play firing sound
    (`/Engine/EditorBlueprintResources/StandardMacros.DecrementInt` (`self.CurrentAmmo`))))

(fn `StartAbsorbing`
  (params (Arms :type "SkeletalMeshComponent Object Reference") (Camera :type "CameraComponent Object Reference"))
  (set `self.PlayerArms` Arms)
  (set `self.PlayerCamera` Camera)
  (`self.SetActorTickEnabled` true))

(fn `StopAbsorbing`
  (`self.SetActorTickEnabled` false)
  (set `self.PlayerArms` null)
  (set `self.PlayerCamera` null))

(fn `UserConstructionScript`)