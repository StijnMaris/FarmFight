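; Health component for FarmFight that tracks current health against a maximum and broadcasts health-changed and death events.
; DoDamage clamps health and ignores hits once dead, and a helper returns health as a fraction.
; Damage over time runs DoDamage on a looping timer, replaced on each start, until stopped or its duration elapses.
; A negative duration runs indefinitely, and the elapsed counter is never reset between runs.
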(event `self.ReceiveBeginPlay`
  (set `self.CurrentHealth` (`self.MaxHealth`)))

(event `StartDOT`
  (params (duration :type "Float (double-precision)") (tickInterval :type "Float (double-precision)") (damagePerTick :type "Float (double-precision)"))
  (set `self.DOTDuration` duration)
  (set `self.DOTTickInterval` tickInterval)
  (set `self.DOTDamagePerTick` damagePerTick)
  (`KismetSystemLibrary.K2_ClearAndInvalidateTimerHandle` (`self.DOTTimerHandle`))
  (bind _returnvalue (`KismetSystemLibrary.K2_SetTimer` null "DoDOTDamage" (`self.DOTTickInterval`) true))
  (set `self.DOTTimerHandle` _returnvalue))

(event `DoDOTDamage`
  (`|ExecutionSequence`
    (:`then_0`
      (`self.DoDamage` (`self.DOTDamagePerTick`)))
    (:`then_1`
      (if (>= (`self.DOTDuration`) 0.0)
        (set `self.DOTDurationTimer` (+ (`self.DOTDurationTimer`) (`self.DOTTickInterval`)))
        (if (>= (`self.DOTDurationTimer`) (`self.DOTDuration`))
          (`KismetSystemLibrary.K2_ClearAndInvalidateTimerHandle` (`self.DOTTimerHandle`)))))))

(event `StopDOT`
  (`KismetSystemLibrary.K2_ClearAndInvalidateTimerHandle` (`self.DOTTimerHandle`)))

(fn `DoDamage`
  (params (incomingDamage :type "Float (double-precision)"))
  (if (not (`self.IsDead`))
    (bind _output_get (set `self.CurrentHealth` (`KismetMathLibrary.FClamp` (- (`self.CurrentHealth`) (`local.incomingDamage`)) 0.0 (`self.MaxHealth`))))
    (`self.OnHealthChangedEvent` _output_get (`self.MaxHealth`))
    (if (`self.IsDead`)
      (`self.OnDiedEvent`))))

(fn `GetCurrentHealthAsAlpha`
  (returns (currentHealthAsAlpha :type "Float (double-precision)"))
  (return (/ (`self.CurrentHealth`) (`self.MaxHealth`))))