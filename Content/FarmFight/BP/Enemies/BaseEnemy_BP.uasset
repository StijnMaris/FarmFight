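; BaseEnemy_BP is an enemy that attacks a list of farm fields in round-robin order.
; A looping timer sends each target a damage-over-time message through HealthInterface, with a duration of -1, then advances the wrapping index.
; Tick runs through a short Delay to steadily damage the enemy's own HealthComponentBP.
; The construction script draws debug lines from ShootLocation to each assigned field.
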(event `self.ReceiveBeginPlay`
  (`KismetSystemLibrary.K2_SetTimer` null "StartDOTOnField" (`self.attackFrequency`) true))

(event `StartDOTOnField`
  (bind _output (`|GetArrayItem` (`self.FarmFieldsToAttack`) (`self.currentTargetIndex`)))
  (`|ExecutionSequence`
    (:`then_0`
      (if (`KismetArrayLibrary.Array_IsValidIndex` (`self.FarmFieldsToAttack`) (`self.currentTargetIndex`))
        (if (`KismetSystemLibrary.DoesImplementInterface` _output "/Game/FarmFight/BP/HealthInterface.HealthInterface_C")
          (message `/Game/FarmFight/BP/HealthInterface.StartDOT` _output -1.0 0.1 1.0))))
    (:`then_1`
      (bind _result (`/Engine/EditorBlueprintResources/StandardMacros.IncrementInt` (`self.currentTargetIndex`))
        (:`  `
          (set `self.currentTargetIndex` (mod _result (`KismetArrayLibrary.Array_Length` (`self.FarmFieldsToAttack`)))))))))

(event `self.ReceiveTick`
  (params (DeltaSeconds :type "Float (single-precision)"))
  (`KismetSystemLibrary.Delay` 0.2)
  (`/Game/FarmFight/BP/HealthComponent_BP.DoDamage` (`self.HealthComponent_BP`) 1.0))

(fn `UserConstructionScript`
  (for _array_element (`self.FarmFieldsToAttack`)
    (`KismetSystemLibrary.DrawDebugLine` (`SceneComponent.K2_GetComponentLocation` (`self.ShootLocation`)) (`self.K2_GetActorLocation` _array_element) (struct :`R` 0.028654 :`G` 1.0 :`A` 1.0) 0.0 5.0)))