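; Base Blueprint for retrievable actors in FarmFight that grow over time until they can be harvested.
; BeginPlay applies the start scale and rotation, then Tick accumulates a timer to linearly interpolate scale toward the end scale over GrowTime.
; Once the timer reaches GrowTime, it sets CanHarvest and disables its own Tick.
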(event `self.ReceiveBeginPlay`
  (`self.SetActorScale3D` (`self.StartScale`))
  (`self.K2_SetActorRotation` (`self.StartRotation`)))

(event `self.ReceiveTick`
  (params (DeltaSeconds :type "Float (single-precision)"))
  (set `self.GrowTimer` (+ DeltaSeconds (`self.GrowTimer`)))
  (`|ExecutionSequence`
    (:`then_0`
      (`self.SetActorScale3D` (`KismetMathLibrary.VLerp` (`self.StartScale`) (`self.EndScale`) (/ (`self.GrowTimer`) (`self.GrowTime`)))))
    (:`then_1`
      (if (>= (`self.GrowTimer`) (`self.GrowTime`))
        (set `self.bCanHarvest` true)
        (`self.SetActorTickEnabled` false)))))

(fn `UserConstructionScript`)