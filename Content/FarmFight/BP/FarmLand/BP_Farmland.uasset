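; BP_Farmland is a farmland actor that fills an area with a grid of spawned actors when play begins.
; BeginPlay derives grid spacing from the Box extent divided by GridSize, then calls CreateGrid.
; CreateGrid runs nested X/Y loops, spawning the class that SpawnType selects from SpawnTypes at positions offset by half the box extent from the actor's location, ignoring collisions.
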(event `self.ReceiveBeginPlay`
  (bind (_gridsize_x _gridsize_y) (`KismetMathLibrary.BreakVector2D` (`self.GridSize`)))
  (bind (_boxextent_x _boxextent_y) (`KismetMathLibrary.BreakVector` (`BoxComponent.BoxExtent` (`self.Box`))))
  (set `self.GridSpacing` (`KismetMathLibrary.MakeVector2D` (/ _boxextent_x _gridsize_x) (/ _boxextent_y _gridsize_y)))
  (`self.CreateGrid`))

(event `CreateGrid`
  (bind (_gridsize_x _gridsize_y) (`KismetMathLibrary.BreakVector2D` (`self.GridSize`)))
  (bind (_gridspacing_x _gridspacing_y) (`KismetMathLibrary.BreakVector2D` (`self.GridSpacing`)))
  (for _index (range (+ (`KismetMathLibrary.Round` _gridsize_x) 1))
    (for _index_2 (range (+ (`KismetMathLibrary.Round` _gridsize_y) 1))
      (`|SpawnActorFromClass` (`|GetArrayItem` (`self.SpawnTypes`) (`KismetMathLibrary.Conv_ByteToInt` (`self.SpawnType`))) (`KismetMathLibrary.MakeTransform` (- (+ (`KismetMathLibrary.MakeVector` (* _index _gridspacing_x) (* _index_2 _gridspacing_y)) (`self.K2_GetActorLocation`)) (* (`BoxComponent.BoxExtent` (`self.Box`)) 0.5))) "AlwaysSpawn" "OverrideRootScale" null null))))

(fn `UserConstructionScript`)