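; Ammo component for FarmFight that tracks a count per ammo ID in a map.
; BeginPlay seeds the map from the starting counts in AmmoDataTable.
; IncrementAmmo clamps between zero and the table's max, then fires the count-changed event, recomputing from the updated map so the increment is applied again in the reported count.
; HasAmmo is true only above one, so a single round reads as empty.
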(event `self.ReceiveBeginPlay`
  (bind _ammodatatable (`self.AmmoDataTable`))
  (bind _outrownames (`DataTableFunctionLibrary.GetDataTableRowNames` _ammodatatable))
  (for _array_element _outrownames
    (bind _returnvalue (`|GetDataTableRow` _ammodatatable _array_element)
      (:`then`
        (`BlueprintMapLibrary.Map_Add` (`self.CurrentAmmo`) _array_element (`.StartingAmmoCount` (break `AmmoTypeDatatableRow` _returnvalue)))))))

(fn `HasAmmo`
  (params (ammoId :type Name))
  (returns (bHasAmmo :type Boolean))
  (bind (_value _returnvalue) (`BlueprintMapLibrary.Map_Find` (`self.CurrentAmmo`) ammoId))
  (if _returnvalue
    (return (> _value 1))
    (else
      (return false))))

(fn `IncrementAmmo`
  (params (ammoId :type Name) (incrementAmount :type Integer))
  (bind (_value _returnvalue) (`BlueprintMapLibrary.Map_Find` (`self.CurrentAmmo`) (`local.ammoId`)))
  (if _returnvalue
    (bind _returnvalue_2 (`|GetDataTableRow` (`self.AmmoDataTable`) (`local.ammoId`))
      (:`then`
        (bind _returnvalue_3 (`KismetMathLibrary.Clamp` (+ _value (`local.incrementAmount`)) 0 (`.MaxAmmoutCount` (break `AmmoTypeDatatableRow` _returnvalue_2))))
        (`BlueprintMapLibrary.Map_Add` (`self.CurrentAmmo`) (`local.ammoId`) _returnvalue_3)
        (`self.OnAmmoCountChangedEvent` (`local.ammoId`) _returnvalue_3)))))